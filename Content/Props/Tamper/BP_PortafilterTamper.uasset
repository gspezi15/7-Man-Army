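; BP_PortafilterTamper is a grabbable tamper prop that tamps coffee grounds in a portafilter.
; When its Box begins overlapping a BP_Portafilter that has grounds and is not yet tampered, it sets that portafilter's Tampered flag.
; When the GrabComponent reports a drop while Hold is true, the tamper snaps to the Tamperlocation of the tamperholder referenced by Tamperhold.
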(event `self.Box.OnComponentBeginOverlap`
  (params (OverlappedComponent :type "PrimitiveComponent Object Reference") (OtherActor :type "Actor Object Reference") (OtherComp :type "PrimitiveComponent Object Reference") (OtherBodyIndex :type Integer) (bFromSweep :type Boolean) (SweepResult :type "HitResult Structure (by ref)"))
  (bind _asbp_portafilter (cast `/Game/Props/Portafilter/BP_Portafilter` OtherActor))
  (if (and (!= (`/Game/Props/Portafilter/BP_Portafilter.Tampered?` _asbp_portafilter) true) (== (`/Game/Props/Portafilter/BP_Portafilter.HasGrounds?` _asbp_portafilter) true))
    (set `/Game/Props/Portafilter/BP_Portafilter.Tampered?` true _asbp_portafilter)))

(event `self.GrabComponent.OnDropped`
  (if (`self.hold`)
    (bind _astamperholder (cast `/Game/Props/tamperholder/tamperholder` (`self.tamperhold`)))
    (`self.K2_SetActorLocation` self (`SceneComponent.K2_GetComponentLocation` (`/Game/Props/tamperholder/tamperholder.tamperlocation` _astamperholder)) false false)))

(fn `UserConstructionScript`)