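; Portafilter prop that tracks whether it holds coffee grounds and whether they are used.
; Fill, use and empty events set these flags, recolor an arrow and print debug messages, with fill and empty also toggling the grounds mesh.
; While grounds are present, Tick reapplies visibility and picks the mesh and material from the Tampered flag, which is only read here.
; RemoveGrounds clears only the grounds flag, leaving visuals unchanged.
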(event `self.ReceiveTick`
  (params (DeltaSeconds :type "Float (single-precision)"))
  (`|ExecutionSequence`
    (:`then_0`
      (`self.IfHasGroundsThenShowGrounds`))))

(event `FillFilter`
  (set `self.HasGrounds?` true)
  (set `self.IsGroundsUsed?` false)
  (`ArrowComponent.SetArrowColor` (`self.Arrow`) (struct :`R` 0.091667 :`G` 0.039586 :`B` 0.003474 :`A` 1.0))
  (`SceneComponent.SetVisibility` (`self.GroundsIndicatorMesh`) true false)
  (`KismetSystemLibrary.PrintString` "Filter Filled"))

(event `UseGrounds`
  (set `self.IsGroundsUsed?` true)
  (`ArrowComponent.SetArrowColor` (`self.Arrow`) (struct :`R` 0.0125 :`G` 0.005993 :`B` 0.002656 :`A` 1.0))
  (`KismetSystemLibrary.PrintString` "Filter Grounds Used"))

(event `EmptyFilter`
  (set `self.HasGrounds?` false)
  (set `self.IsGroundsUsed?` false)
  (`SceneComponent.SetVisibility` (`self.GroundsIndicatorMesh`) false false)
  (`ArrowComponent.SetArrowColor` (`self.Arrow`) (struct :`G` 1.0 :`A` 1.0))
  (`KismetSystemLibrary.PrintString` "Filter Emptied"))

(fn `IfHasGroundsThenShowGrounds`
  (bind _groundsindicatormesh (`self.GroundsIndicatorMesh`))
  (if (`self.HasGrounds?`)
    (`|ExecutionSequence`
      (:`then_0`
        (`SceneComponent.SetVisibility` (`self.GroundsIndicatorMesh`) true false))
      (:`then_1`
        (if (`self.Tampered?`)
          (`StaticMeshComponent.SetStaticMesh` _groundsindicatormesh "/Game/Props/coffeegranules/tamperedcoffee.tamperedcoffee")
          (`PrimitiveComponent.SetMaterial` (`self.GroundsIndicatorMesh`) 0 "/Game/Props/coffeegranules/tamperedcoffeegranule.tamperedcoffeegranule")
          (else
            (`StaticMeshComponent.SetStaticMesh` _groundsindicatormesh "/Game/Props/coffeegranules/untamperedcoffee.untamperedcoffee")
            (`PrimitiveComponent.SetMaterial` (`self.GroundsIndicatorMesh`) 0 "/Game/Props/coffeegranules/coffeegranule.coffeegranule")))))))

(fn `Remove_Grounds`
  (if (`self.HasGrounds?`)
    (set `self.HasGrounds?` false)))

(fn `UserConstructionScript`)