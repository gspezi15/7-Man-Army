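; VR coffee machine prop that fills cups with espresso or water and snaps its portafilter into place on overlap.
; Brew and water events sphere-trace below an arrow for a BP_Cup, add liquid in delayed steps, then reset the VR_Button.
; Hand-tagged overlaps play button sequences, whose events set states that Tick shows through material swaps.
; The steam event is empty, and older brew-loop logic is disconnected.
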(event `self.ReceiveTick`
  (params (DeltaSeconds :type "Float (single-precision)"))
  (`|ExecutionSequence`
    (:`then_0`
      (`self.coffeebuttoncolourchange`))
    (:`then_1`
      (`self.steamwandcolourchange`))))

(event `self.makecoffeecollision.OnComponentBeginOverlap`
  (params (OverlappedComponent :type "PrimitiveComponent Object Reference") (OtherActor :type "Actor Object Reference") (OtherComp :type "PrimitiveComponent Object Reference") (OtherBodyIndex :type Integer) (bFromSweep :type Boolean) (SweepResult :type "HitResult Structure (by ref)"))
  (if (`ActorComponent.ComponentHasTag` OtherComp "hand")
    (`MovieSceneSequencePlayer.Play` (`ActorSequenceComponent.SequencePlayer` (`self.coffeebuttonpress`)))))

(event `self.makecoffeecollision.OnComponentEndOverlap`
  (params (OverlappedComponent :type "PrimitiveComponent Object Reference") (OtherActor :type "Actor Object Reference") (OtherComp :type "PrimitiveComponent Object Reference") (OtherBodyIndex :type Integer))
  (if (`ActorComponent.ComponentHasTag` OtherComp "hand")
    (`MovieSceneSequencePlayer.PlayReverse` (`ActorSequenceComponent.SequencePlayer` (`self.coffeebuttonrelease`)))))

(event `self.steamwandcollision.OnComponentBeginOverlap`
  (params (OverlappedComponent :type "PrimitiveComponent Object Reference") (OtherActor :type "Actor Object Reference") (OtherComp :type "PrimitiveComponent Object Reference") (OtherBodyIndex :type Integer) (bFromSweep :type Boolean) (SweepResult :type "HitResult Structure (by ref)"))
  (if (`ActorComponent.ComponentHasTag` OtherComp "hand")
    (`MovieSceneSequencePlayer.Play` (`ActorSequenceComponent.SequencePlayer` (`self.steamwandbuttonpress`)))))

(event `self.steamwandcollision.OnComponentEndOverlap`
  (params (OverlappedComponent :type "PrimitiveComponent Object Reference") (OtherActor :type "Actor Object Reference") (OtherComp :type "PrimitiveComponent Object Reference") (OtherBodyIndex :type Integer))
  (if (`ActorComponent.ComponentHasTag` OtherComp "hand")
    _))

(event `self.ReceiveBeginPlay`)

(event `EventBrew`
  (bind _returnvalue (`SceneComponent.GetSocketLocation` (`self.Arrow`) "None"))
  (bind _outhit (`KismetSystemLibrary.SphereTraceSingle` :`Start` _returnvalue :`End` (- _returnvalue (0.0 0.0 40.0)) :`Radius` 9.0 :`TraceChannel` "TraceTypeQuery1" :`DrawDebugType` "ForDuration"))
  (bind _asbp_cup (cast `/Game/Props/cups/BP_Cup` (`.HitActor` (`GameplayStatics.BreakHitResult` _outhit)))
    (:`then`
      (set `self.CurrentCup` _asbp_cup)
      (`|SpawnActorFromClass` "/Game/CoffeeCustomBP/Temp_LiquidMockup.Temp_LiquidMockup_C" (`KismetMathLibrary.MakeTransform` (`SceneComponent.K2_GetComponentLocation` (`/Game/Props/cups/BP_Cup.StaticMesh` _asbp_cup))) "Undefined" "OverrideRootScale" null null)
      (`GameplayStatics.PlaySound2D` "/Game/Audio/658711__tlabrant1__pouring-a-cup-of-coffee.658711__tlabrant1__pouring-a-cup-of-coffee" 1.0 1.0 0.0 null null)
      (`self.Macro_SimplifiedBrew`
        (:`NewParam2`
          (bind _asvr_button (cast `/Game/CoffeeCustomBP/VR_Button` (`self.LastActivatorButton`)))
          (`/Game/CoffeeCustomBP/VR_Button.ResetButton` _asvr_button))))
    (:`CastFailed`
      (`KismetSystemLibrary.PrintString` "CoffeeMachine cast to cup failed" true true (struct :`R` 0.988 :`A` 1.0) 3.0)
      (bind _asvr_button_2 (cast `/Game/CoffeeCustomBP/VR_Button` (`self.LastActivatorButton`)))
      (`/Game/CoffeeCustomBP/VR_Button.ResetButton` _asvr_button_2))))

(event `self.Box.OnComponentBeginOverlap`
  (params (OverlappedComponent :type "PrimitiveComponent Object Reference") (OtherActor :type "Actor Object Reference") (OtherComp :type "PrimitiveComponent Object Reference") (OtherBodyIndex :type Integer) (bFromSweep :type Boolean) (SweepResult :type "HitResult Structure (by ref)"))
  (bind _childactor (`ChildActorComponent.ChildActor` (`self.portaf`)))
  (cast `/Game/Props/Portafilter/BP_Portafilter` _childactor)
  (`self.K2_SetActorLocationAndRotation` :`self` _childactor :`NewLocation` (`SceneComponent.K2_GetComponentLocation` (`self.portoGoTo`))))

(event `EventWater`
  (bind _returnvalue (`SceneComponent.GetSocketLocation` (`self.Arrow`) "None"))
  (bind _outhit (`KismetSystemLibrary.SphereTraceSingle` _returnvalue (- _returnvalue (0.0 0.0 40.0)) 10.0 "TraceTypeQuery1"))
  (bind _asbp_cup (cast `/Game/Props/cups/BP_Cup` (`.HitActor` (`GameplayStatics.BreakHitResult` _outhit)))
    (:`then`
      (set `self.CurrentCup` _asbp_cup)
      (`self.Macro_SimplifiedWater`
        (:`NewParam2`
          (bind _asvr_button (cast `/Game/CoffeeCustomBP/VR_Button` (`self.LastActivatorButton`)))
          (`/Game/CoffeeCustomBP/VR_Button.ResetButton` _asvr_button))))
    (:`CastFailed`
      (`KismetSystemLibrary.PrintString` "CoffeeMachine cast to cup failed" true true (struct :`R` 0.988 :`A` 1.0) 3.0)
      (bind _asvr_button_2 (cast `/Game/CoffeeCustomBP/VR_Button` (`self.LastActivatorButton`)))
      (`/Game/CoffeeCustomBP/VR_Button.ResetButton` _asvr_button_2))))

(event `EventSteam`)

(event `coffeebuttonmodel_Event_0`
  (params (coffeebuttonmodel :type "StaticMeshComponent Object Reference"))
  (if (`self.MakeCoffeeButtonOn`)
    (set `self.MakeCoffeeButtonOn` false)
    (else
      (set `self.MakeCoffeeButtonOn` true))))

(event `activatesteamwand`
  (params (Owner :type "Actor Object Reference"))
  (set `self.SteamWandActivate` true))

(event `deactivatesteamwand`
  (params (Owner :type "Actor Object Reference"))
  (set `self.SteamWandActivate` false))

(fn `BrewEspressoCup`
  (bind _asbp_cup (cast `/Game/Props/cups/BP_Cup` (`self.CurrentCup`)))
  (if (not (>= (`/Game/Props/cups/BP_Cup.AmountEspresso` _asbp_cup) 20))
    (bind _asbp_cup_2 (cast `/Game/Props/cups/BP_Cup` (`self.CurrentCup`)))
    (bind _output_get (set `/Game/Props/cups/BP_Cup.AmountEspresso` (`KismetMathLibrary.Clamp` (+ (`/Game/Props/cups/BP_Cup.AmountEspresso` _asbp_cup_2) 1) 0 20) _asbp_cup_2))
    (`KismetSystemLibrary.PrintString` (`KismetStringLibrary.Conv_IntToString` _output_get))
    (return)))

(fn `coffeebuttoncolourchange`
  (bind _coffeebuttonmodel (`self.coffeebuttonmodel`))
  (if (`self.MakeCoffeeButtonOn`)
    (`PrimitiveComponent.SetMaterial` _coffeebuttonmodel 0 "/Game/Props/CoffeeMachine/material/coffeebuttongreen.coffeebuttongreen")
    (else
      (`PrimitiveComponent.SetMaterial` _coffeebuttonmodel 0 "/Game/Props/CoffeeMachine/material/coffeebuttonred.coffeebuttonred"))))

(fn `steamwandcolourchange`
  (bind _steamwandbutton (`self.steamwandbutton`))
  (if (`self.SteamWandActivate`)
    (`PrimitiveComponent.SetMaterial` _steamwandbutton 0 "/Game/Props/CoffeeMachine/material/onsteamwandbutton_Mat.onsteamwandbutton_Mat")
    (else
      (`PrimitiveComponent.SetMaterial` _steamwandbutton 0 "/Game/Props/CoffeeMachine/material/offsteamwandbutton_Mat.offsteamwandbutton_Mat"))))

(fn `UserConstructionScript`)