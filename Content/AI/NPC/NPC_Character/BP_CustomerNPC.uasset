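; BP_CustomerNPC is a customer NPC character that can pick a random coffee order and display it on a widget component.
; SelectRandomCoffeeOrder rolls one of four coffee types, prints debug text, then creates the matching widget class through parallel CoffeeOrderType and CoffeeWidget arrays.
; The printed number comes from a pure random node, so it can differ from the order.
; BeginPlay is empty and the event graph's order call is unwired.
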(event `self.ReceiveBeginPlay`)

(fn `SelectRandomCoffeeOrder`
  (bind _returnvalue (`KismetMathLibrary.Conv_IntToByte` (`KismetMathLibrary.RandomIntegerInRange` 0 3)))
  (bind _output_get (set `self.CoffeeOrder` (cast `/Game/CoffeeCustomBP/CoffeeType_Enum` _returnvalue)))
  (bind _output (`|GetArrayItem` (`self.CoffeeWidget`) (`KismetArrayLibrary.Array_Find` (`self.CoffeeOrderType`) _output_get)))
  (`KismetSystemLibrary.PrintString` (`KismetStringLibrary.Concat_StrStr` "Order" (`|GetEnumeratorNameAsString` _output_get) (`KismetStringLibrary.Conv_IntToString` (`KismetMathLibrary.Conv_ByteToInt` _returnvalue)) (`KismetSystemLibrary.GetClassDisplayName` _output) (`KismetSystemLibrary.GetDisplayName` self)) true true (struct :`G` 0.66 :`B` 1.0 :`A` 1.0) 5.0)
  (bind _returnvalue_2 (`|CreateWidget` _output))
  (`WidgetComponent.SetWidget` (`self.Widget`) _returnvalue_2))

(fn `UserConstructionScript`)