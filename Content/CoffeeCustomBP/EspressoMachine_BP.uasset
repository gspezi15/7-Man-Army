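; Espresso machine actor that turns a DrinkCup_BP into an espresso drink.
; When an actor overlaps its box, a cup gets its drink type set, its espresso amount topped up to a cap and its debug text refreshed.
; Machine_Activate sphere-traces down from the arrow, then runs the same fill logic on the overlap's OtherActor, ignoring the trace result.
; Debug strings report each outcome.
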(event `self.Box.OnComponentBeginOverlap`
  (params (OverlappedComponent :type "PrimitiveComponent Object Reference") (OtherActor :type "Actor Object Reference") (OtherComp :type "PrimitiveComponent Object Reference") (OtherBodyIndex :type Integer) (bFromSweep :type Boolean) (SweepResult :type "HitResult Structure (by ref)"))
  (`KismetSystemLibrary.PrintString` "Something has touched the box")
  (bind _asdrink_cup_bp (cast `/Game/CoffeeCustomBP/DrinkCup_BP` OtherActor :!label _label)
    (:`then`
      (set `/Game/CoffeeCustomBP/DrinkCup_BP.DrinkType` "NewEnumerator1" _asdrink_cup_bp)
      (set `/Game/CoffeeCustomBP/DrinkCup_BP.AmountEspresso` (`KismetMathLibrary.Clamp` (+ (`/Game/CoffeeCustomBP/DrinkCup_BP.AmountEspresso` _asdrink_cup_bp) 20) 0 20) _asdrink_cup_bp)
      (`/Game/CoffeeCustomBP/DrinkCup_BP.UpdateDebugDrinkTypeText` _asdrink_cup_bp)
      (`KismetSystemLibrary.PrintString` "\"Now Give Me Coffee aand TV....\""))
    (:`CastFailed`
      (`KismetSystemLibrary.PrintString` "This Aint a cup"))))

(event `Machine_Activate`
  (bind _returnvalue (`SceneComponent.K2_GetComponentLocation` (`self.Arrow`)))
  (`KismetSystemLibrary.SphereTraceSingle` :`Start` _returnvalue :`End` (- _returnvalue (0.0 0.0 60.0)) :`TraceChannel` "TraceTypeQuery1" :`DrawDebugType` "ForDuration")
  (goto _label))

(fn `UserConstructionScript`)