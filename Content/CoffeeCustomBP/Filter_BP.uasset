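; Coffee filter Blueprint that tracks whether it holds grounds and whether those grounds have been used.
; Three events, to fill, use and empty the filter, set the two state flags without checking the current state.
; An Arrow component's color shows the state (brown for fresh, darker brown for used, green for empty), and each event prints a message.
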(event `FillFilter`
  (set `self.HasGrounds?` true)
  (set `self.IsGroundsUsed?` false)
  (`ArrowComponent.SetArrowColor` (`self.Arrow`) (struct :`R` 0.091667 :`G` 0.039586 :`B` 0.003474 :`A` 1.0))
  (`KismetSystemLibrary.PrintString` "Filter Filled"))

(event `UseGrounds`
  (set `self.IsGroundsUsed?` true)
  (`ArrowComponent.SetArrowColor` (`self.Arrow`) (struct :`R` 0.0125 :`G` 0.005993 :`B` 0.002656 :`A` 1.0))
  (`KismetSystemLibrary.PrintString` "Filter Grounds Used"))

(event `EmptyFilter`
  (set `self.HasGrounds?` false)
  (set `self.IsGroundsUsed?` false)
  (`ArrowComponent.SetArrowColor` (`self.Arrow`) (struct :`G` 1.0 :`A` 1.0))
  (`KismetSystemLibrary.PrintString` "Filter Emptied"))

(fn `UserConstructionScript`)